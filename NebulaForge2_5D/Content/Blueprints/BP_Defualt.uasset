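; BP_Defualt is a player-controlled 2D Paper archer character for a side-view platformer, with health, melee attack, dash, double jump and void teleport.
; Enhanced Input drives movement and abilities; Tick selects movement flipbooks through UpdateAnim.
; Attacks fire HitCheck once at flipbook frame 4 via DoOnce, damaging overlapping BP_Defualt actors.
; HasVoidTelport gates teleporting to a fixed location, while HasDash and HasDoubleJump checks are disconnected.
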(event Custom|Reset%20Attack
  (Utilities|FlowControl|DoOnce false) ; enters at Reset
)

(event Input|EnhancedActionEvents|EnhancedInputActionIA_Jump
  (params (ActionValue :type Boolean) (ElapsedSeconds :type Float%20%28double-precision%29) (TriggeredSeconds :type Float%20%28double-precision%29) (InputAction :type Input%20Action%20Object%20Reference :default "/Game/Input/Actions/IA_Jump.IA_Jump"))
  (:Started
    (Character|Jump)
    (if (AI|Components|NavMovement|IsFalling (Variables|Character|GetCharacterMovement))
      (if (not (Variables|Default|GetIs%20Double%20Jumping))
        (Variables|Default|SetIs%20Double%20Jumping true)
        (Character|LaunchCharacter "0.000000,0.000000,850.000000" false false)
        (Utilities|FlowControl|Delay 0.5)
        (Variables|Default|SetIs%20Double%20Jumping false))))
  (:Completed
    (Character|StopJumping)))

(event Input|EnhancedActionEvents|EnhancedInputActionIA_Dash
  (params (ActionValue :type Boolean) (ElapsedSeconds :type Float%20%28double-precision%29) (TriggeredSeconds :type Float%20%28double-precision%29) (InputAction :type Input%20Action%20Object%20Reference :default "/Game/Input/Actions/IA_Dash.IA_Dash"))
  (bind _returnvalue (Transformation|GetVelocity))
  (bind _returnvalue_2 (* _returnvalue 1e+01))
  (if (not (Variables|Default|GetIsDashing))
    (Variables|Default|SetIsDashing true)
    (Character|LaunchCharacter (Math|Vector|MakeVector (.x _returnvalue_2) (.y _returnvalue_2) 0.0) false false)
    (Utilities|FlowControl|Delay 0.5)
    (Variables|Default|SetIsDashing false)))

(event Input|EnhancedActionEvents|EnhancedInputActionIA_Attack
  (params (ActionValue :type Boolean) (ElapsedSeconds :type Float%20%28double-precision%29) (TriggeredSeconds :type Float%20%28double-precision%29) (InputAction :type Input%20Action%20Object%20Reference :default "/Game/Input/Actions/IA_Attack.IA_Attack"))
  (Sprite|SetFlipbook (Variables|Default|GetSprite) "/Game/Sprites/Acher/FlipBooks/ArcherATTACK.ArcherATTACK")
  (Components|Timeline|SetLooping (Variables|Default|GetSprite) true)
  (Variables|Default|SetIsAtacking? true)
  (Audio|PlaySound2D 0 1.0 1.0 0.0 0 0)
  (Utilities|FlowControl|Delay 0.8)
  (if (not (Variables|Default|GetIsDead))
    (Sprite|SetFlipbook (Variables|Default|GetSprite) "/Game/Sprites/Acher/FlipBooks/ArcherIDLE.ArcherIDLE")
    (Variables|Default|SetIsAtacking? false)
    (CallFunction|ResetAttack)
    (Development|SetHiddeninGame (Variables|Default|GetHitbox) true false)))

(event Input|EnhancedActionEvents|EnhancedInputActionIA_VoidTeleport
  (params (ActionValue :type Boolean) (ElapsedSeconds :type Float%20%28double-precision%29) (TriggeredSeconds :type Float%20%28double-precision%29) (InputAction :type Input%20Action%20Object%20Reference :default "/Game/Input/Actions/IA_VoidTeleport.IA_VoidTeleport"))
  (if (Variables|Default|GetHasVoidTelport)
    (Transformation|Teleport "21860.000000,0.000000,-3570.000000" "0, 0, 0")))

(event Input|EnhancedActionEvents|EnhancedInputActionIA_Move
  (params (ActionValue :type Float%20%28double-precision%29) (ElapsedSeconds :type Float%20%28double-precision%29) (TriggeredSeconds :type Float%20%28double-precision%29) (InputAction :type Input%20Action%20Object%20Reference :default "/Game/Input/Actions/IA_Move.IA_Move"))
  (Pawn|Input|AddMovementInput "0.800000,0.000000,0.000000" ActionValue false)
  (Pawn|SetControlRotation (Pawn|GetController) (select (> ActionValue 0.0) (Math|Rotator|MakeRotator 0.0 0.0 0.0) (Math|Rotator|MakeRotator 0.0 0.0 1.8e+02))))

(event EventBeginPlay
  (bind _asplayer_controller (Utilities|Casting|CastToPlayerController (Pawn|GetController)))
  (Input|AddMappingContext (PlayerController|LocalPlayerSubsystems|GetEnhancedInputLocalPlayerSubsystem _asplayer_controller) "/Game/Input/IMC_Platforming.IMC_Platforming" 0 "(bIgnoreAllPressedKeysUntilRelease=True,bForceImmediately=False,bNotifyUserSettings=False)"))

(event Collision|EventActorBeginOverlap
  (params (OtherActor :type Actor%20Object%20Reference)))

(event EventTick
  (params (DeltaSeconds :type Float%20%28single-precision%29))
  (CallFunction|UpdateAnim)
  (if (Variables|Default|GetIsAtacking?)
    (if (== (Class|PaperFlipbookComponent|GetPlaybackPositioninFrames (Variables|Default|GetSprite)) 4)
      (Utilities|FlowControl|DoOnce false
        (:Completed
          (CallFunction|HitCheck)
          (Development|SetHiddeninGame (Variables|Default|GetHitbox) false false))))
    (else
      (Development|SetHiddeninGame (Variables|Default|GetHitbox) true false))))

(event Game|Damage|EventAnyDamage
  (params (Damage :type Float%20%28single-precision%29) (DamageType :type Damage%20Type%20Object%20Reference) (InstigatedBy :type Controller%20Object%20Reference) (DamageCauser :type Actor%20Object%20Reference))
  (Variables|Default|SetHealth (- (Variables|Default|GetHealth) Damage))
  (if (<= (Variables|Default|GetHealth) 0.0)
    (Sprite|SetFlipbook (Variables|Default|GetSprite) "/Game/Sprites/Acher/FlipBooks/ArcherDEATH.ArcherDEATH")
    (Components|Timeline|SetLooping (Variables|Default|GetSprite) false)
    (Variables|Default|SetIsDead true)
    (else
      (Sprite|SetFlipbook (Variables|Default|GetSprite) "/Game/Sprites/Acher/FlipBooks/Archer_TakeDamge.Archer_TakeDamge")
      (Components|Timeline|SetLooping (Variables|Default|GetSprite) false))))

(fn ConstructionScript)

(fn UpdateAnim
  (if (not (Variables|Default|GetIsAtacking?))
    (if (AI|Components|NavMovement|IsMovingonGround (Variables|Character|GetCharacterMovement))
      (if (> (Math|Vector|VectorLength (Transformation|GetVelocity)) 0.0)
        (Sprite|SetFlipbook (Variables|Default|GetSprite) "/Game/Sprites/Acher/FlipBooks/ArcherWALK.ArcherWALK")
        (else
          (Sprite|SetFlipbook (Variables|Default|GetSprite) "/Game/Sprites/Acher/FlipBooks/ArcherIDLE.ArcherIDLE")))
      (elif (< (.z (Transformation|GetVelocity)) -1e+02)
        (Sprite|SetFlipbook (Variables|Default|GetSprite) "/Game/Sprites/Acher/FlipBooks/ArcherJUMPFALL.ArcherJUMPFALL")
        (else
          (Sprite|SetFlipbook (Variables|Default|GetSprite) "/Game/Sprites/Acher/FlipBooks/ArcherJUMPRISE.ArcherJUMPRISE"))))))

(fn HitCheck
  (for _array_element (Collision|GetOverlappingActors (Variables|Default|GetHitbox) "BP_Defualt_C" :!class /Script/Engine.PrimitiveComponent)
    (if (!= _array_element self)
      (Game|Damage|ApplyDamage _array_element (Variables|Default|GetDamge%20Amount) 0 0)
      (LocalVariables|SetHit%20Somthing true)))
  (if (LocalVariables|GetHit%20Somthing)
    (Effects|SpawnEmitteratLocation "/Game/Particles_Wind_Control_System/Blueprints/Components/Particles/P_Fireflies.P_Fireflies" (Transformation|GetSocketLocation (Variables|Default|GetSprite) "HitPos"))
    (Audio|PlaySound2D 0 1.0 1.0 0.0 0 0)))