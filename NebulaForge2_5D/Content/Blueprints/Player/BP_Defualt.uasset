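; Player character for a 2D flipbook platformer, with Enhanced Input movement, dash, double jump, melee attack, hold-to-heal, gated void teleport and NPC dialogue via interface.
; Tick runs ResetAttack1, which checks health to open a level on death, updates flipbooks and applies hitbox damage on an attack frame.
; SpawnArrow repositions an existing Arrow actor beneath the player as a mid-double-jump platform.
; Dash and double-jump unlock checks are disconnected.
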(event Input|EnhancedActionEvents|EnhancedInputActionIA_Jump
  (params (ActionValue :type Boolean) (ElapsedSeconds :type Float%20%28double-precision%29) (TriggeredSeconds :type Float%20%28double-precision%29) (InputAction :type Input%20Action%20Object%20Reference :default "/Game/Input/Actions/IA_Jump.IA_Jump"))
  ;[1 1 1] _Jump && DoubleJump
  (:Started
    (Character|Jump)
    (if (AI|Components|NavMovement|IsFalling (Variables|Character|GetCharacterMovement))
      (if (not (Variables|Default|GetIs%20Double%20Jumping))
        (Variables|Default|SetIs%20Double%20Jumping true)
        (Character|LaunchCharacter "0.000000,0.000000,600.000000" false false)
        (Utilities|FlowControl|Delay 0.5)
        (Variables|Default|SetIs%20Double%20Jumping false))))
  (:Completed
    (Character|StopJumping)))

(event Input|EnhancedActionEvents|EnhancedInputActionIA_Dash
  (params (ActionValue :type Boolean) (ElapsedSeconds :type Float%20%28double-precision%29) (TriggeredSeconds :type Float%20%28double-precision%29) (InputAction :type Input%20Action%20Object%20Reference :default "/Game/Input/Actions/IA_Dash.IA_Dash"))
  (bind _returnvalue (Transformation|GetVelocity))
  (bind _returnvalue_2 (Transformation|GetVelocity))
  (bind _dashpower (Variables|Default|GetDashPower))
  (bind _dashpower_2 (Variables|Default|GetDashPower))
  (bind _returnvalue_3 (+ _returnvalue_2 _dashpower_2))
  (bind _returnvalue_4 (- _returnvalue _dashpower))
  ;[1 1 1] _Dash
  (if (not (Variables|Default|GetIsDashing))
    (if (== (.yaw (Transformation|GetActorRotation)) 1.8e+02)
      (Variables|Default|SetIsDashing true)
      (Character|LaunchCharacter (Math|Vector|MakeVector (.x _returnvalue_4) (.y _returnvalue_4) 0.0) false false)
      (Utilities|FlowControl|Delay (Variables|Default|GetDashLength))
      (Variables|Default|SetIsDashing false)
      (else
        (Variables|Default|SetIsDashing true)
        (Character|LaunchCharacter (Math|Vector|MakeVector (.x _returnvalue_3) (.y _returnvalue_3) 0.0) false false)
        (Utilities|FlowControl|Delay (Variables|Default|GetDashLength))
        (Variables|Default|SetIsDashing false)))))

(event Input|EnhancedActionEvents|EnhancedInputActionIA_Attack
  (params (ActionValue :type Boolean) (ElapsedSeconds :type Float%20%28double-precision%29) (TriggeredSeconds :type Float%20%28double-precision%29) (InputAction :type Input%20Action%20Object%20Reference :default "/Game/Input/Actions/IA_Attack.IA_Attack"))
  ;[1 1 1] _Attack
  (Variables|Default|SetIsAtacking? true)
  (Sprite|SetFlipbook (Variables|Default|GetSprite) "/Game/Blueprints/Player/Bosses/Royal_Executioner/Pixel/Sprites/Attack_Simple/Attack1_Combo.Attack1_Combo")
  (Components|Timeline|SetLooping (Variables|Default|GetSprite) true)
  (Audio|PlaySound2D 0 1.0 1.0 0.0 0 0)
  (Utilities|FlowControl|Delay 0.8)
  (if (not (Variables|Default|GetIsDead))
    (Sprite|SetFlipbook (Variables|Default|GetSprite) "/Game/Blueprints/Player/Bosses/Royal_Executioner/Pixel/Sprites/Idle/Idle1.Idle1")
    (Variables|Default|SetIsAtacking? false)
    (CallFunction|ResetAttack1)
    (Development|SetHiddeninGame (Variables|Default|GetHitbox) true false)))

(event Input|EnhancedActionEvents|EnhancedInputActionIA_VoidTeleport
  (params (ActionValue :type Boolean) (ElapsedSeconds :type Float%20%28double-precision%29) (TriggeredSeconds :type Float%20%28double-precision%29) (InputAction :type Input%20Action%20Object%20Reference :default "/Game/Input/Actions/IA_VoidTeleport.IA_VoidTeleport"))
  ;[1 1 1] _Voidteleport
  (CallFunction|VoidTP))

(event Input|EnhancedActionEvents|EnhancedInputActionIA_Move
  (params (ActionValue :type Float%20%28double-precision%29) (ElapsedSeconds :type Float%20%28double-precision%29) (TriggeredSeconds :type Float%20%28double-precision%29) (InputAction :type Input%20Action%20Object%20Reference :default "/Game/Input/Actions/IA_Move.IA_Move"))
  ;[1 1 1] _Movement && Flip
  (CallFunction|Movement ActionValue ActionValue))

(event Input|EnhancedActionEvents|EnhancedInputActionIA_Crouch
  (params (ActionValue :type Boolean) (ElapsedSeconds :type Float%20%28double-precision%29) (TriggeredSeconds :type Float%20%28double-precision%29) (InputAction :type Input%20Action%20Object%20Reference :default "/Game/IA_Crouch.IA_Crouch"))
  (:Completed
    (if (Variables|Default|GetCrouching)
      (Variables|Default|SetCrouching false)
      (else
        (Variables|Default|SetCrouching true)))))

(event EventBeginPlay
  ;[1 1 1] _Inputs
  (CallFunction|Inputs))

(event EventTick
  (params (DeltaSeconds :type Float%20%28single-precision%29))
  ;[1 1 1] _UpdateAnim && Attack && IsTouchingGround
  (CallFunction|ResetAttack1)
  (if (Variables|Default|GetCanLeave)
    (CallFunction|SpawnArrow)))

(event Game|Damage|EventAnyDamage
  (params (Damage :type Float%20%28single-precision%29) (DamageType :type Damage%20Type%20Object%20Reference) (InstigatedBy :type Controller%20Object%20Reference) (DamageCauser :type Actor%20Object%20Reference))
  ;[1 1 1] _Damage
  (CallFunction|Damage Damage (Variables|Default|GetSprite)))

(event Input|KeyboardEvents|F
  (params (Key :type Key%20Structure :default "None"))
  ;[1 1 1] _Heal(BETA)
  (:Pressed
    (Utilities|FlowControl|Delay 2.0)
    (Variables|Default|SethealReady true))
  (:Released
    (if (Variables|Default|GethealReady)
      (Variables|Default|SetHealth (+ (Variables|Default|GetHealth) 1)))))

(event Input|KeyboardEvents|W
  (params (Key :type Key%20Structure :default "None"))
  ;[1 1 1] _TavernKeepInteractions
  (:Pressed
    (for _array_element (Collision|GetOverlappingActors "/Game/Blueprints/Player/Village_NPCS/TavernKeeper/TavernKeeper.TavernKeeper_C" :!class /Script/Engine.Actor)
      (if (Utilities|DoesObjectImplementInterface _array_element "/Game/Blueprints/Dialoouge/BPI_Dialougue.BPI_Dialougue_C")
        (Class|BPIDialougue|Talk(Message) _array_element)))))

(event Input|KeyboardEvents|W
  (params (Key :type Key%20Structure :default "None"))
  ;[1 1 1] _Wizard_Interactions
  (:Pressed
    (for _array_element (Collision|GetOverlappingActors "/Game/Blueprints/Player/Bosses/Riddler/Green_Wizard_DoubleJump.Green_Wizard_DoubleJump_C" :!class /Script/Engine.Actor)
      (if (Utilities|DoesObjectImplementInterface _array_element "/Game/Blueprints/Dialoouge/BPI_Dialougue.BPI_Dialougue_C")
        (Class|BPIDialougue|Talk(Message) _array_element)))))

(event Input|KeyboardEvents|W
  (params (Key :type Key%20Structure :default "None"))
  ;[1 1 1] _Wizard_Interactions
  (:Pressed
    (for _array_element (Collision|GetOverlappingActors "/Game/Blueprints/Player/Bosses/Riddler/Green_Wizard_Dash.Green_Wizard_Dash_C" :!class /Script/Engine.Actor)
      (if (Utilities|DoesObjectImplementInterface _array_element "/Game/Blueprints/Dialoouge/BPI_Dialougue.BPI_Dialougue_C")
        (Class|BPIDialougue|Talk(Message) _array_element)))))

(event Input|KeyboardEvents|E
  (params (Key :type Key%20Structure :default "None"))
  (:Pressed
    (Variables|Default|SetPlacePLatform true)
    (Utilities|FlowControl|Delay 0.2)
    (Variables|Default|SetPlacePLatform false)))

(fn ConstructionScript)

(fn UpdateAnim
  (if (not (Variables|Default|GetIsAtacking?))
    (if (AI|Components|NavMovement|IsMovingonGround (Variables|Character|GetCharacterMovement))
      (if (> (Math|Vector|VectorLength (Transformation|GetVelocity)) 0.0)
        (Sprite|SetFlipbook (Variables|Default|GetSprite) "/Game/Blueprints/Player/Bosses/Royal_Executioner/Pixel/Sprites/Run/Run1.Run1")
        (else
          (Sprite|SetFlipbook (Variables|Default|GetSprite) "/Game/Blueprints/Player/Bosses/Royal_Executioner/Pixel/Sprites/Idle/Idle1.Idle1")))
      (elif (< (.z (Transformation|GetVelocity)) -1e+02)
        (Sprite|SetFlipbook (Variables|Default|GetSprite) "/Game/Blueprints/Player/Bosses/Royal_Executioner/Pixel/Random/JumpRise_Flipbook.JumpRise_Flipbook")
        (else
          (Sprite|SetFlipbook (Variables|Default|GetSprite) "/Game/Blueprints/Player/Bosses/Royal_Executioner/Pixel/Random/JumpFall.JumpFall"))))))

(fn HitCheck
  (for _array_element (Collision|GetOverlappingActors (Variables|Default|GetHitbox) "BP_Defualt_C" :!class /Script/Engine.PrimitiveComponent)
    (if (!= _array_element self)
      (Game|Damage|ApplyDamage _array_element (Variables|Default|GetDamge%20Amount) 0 0)
      (LocalVariables|SetHit%20Somthing true)))
  (if (LocalVariables|GetHit%20Somthing)
    (Effects|SpawnEmitteratLocation 0 (Transformation|GetSocketLocation (Variables|Default|GetSprite) "HitPos"))
    (Audio|PlaySound2D 0 1.0 1.0 0.0 0 0)))

(fn CheckHealth
  (if (< (Variables|Default|GetHealth) 1)
    (Game|OpenLevel(byObjectReference) "/Game/Pixel/Maps/M_2D_Fix.M_2D_Fix")))

(fn ResetAttack1
  (CallFunction|CheckHealth)
  (CallFunction|UpdateAnim)
  (if (Variables|Default|GetIsAtacking?)
    (CallFunction|SpawnArrow)
    (if (== (Class|PaperFlipbookComponent|GetPlaybackPositioninFrames (Variables|Default|GetSprite)) 4)
      (Utilities|FlowControl|DoOnce false
        (:Completed
          (CallFunction|HitCheck)
          (Development|SetHiddeninGame (Variables|Default|GetHitbox) false false)
          (if (== (.z (Transformation|GetVelocity)) 0.0)
            (Variables|Default|SetIsTouchingGround true)
            (else
              (Variables|Default|SetIsTouchingGround false))))))
    (else
      (Development|SetHiddeninGame (Variables|Default|GetHitbox) true false))))

(fn Inputs
  (bind _asplayer_controller (Utilities|Casting|CastToPlayerController (Pawn|GetController)))
  (Input|AddMappingContext (PlayerController|LocalPlayerSubsystems|GetEnhancedInputLocalPlayerSubsystem _asplayer_controller) "/Game/Input/IMC_Platforming.IMC_Platforming" 0 "(bIgnoreAllPressedKeysUntilRelease=True,bForceImmediately=False,bNotifyUserSettings=False)")
  (bind _returnvalue (UserInterface|CreateWidget "/Game/Blueprints/Widgets/Health.Health_C"))
  (UserInterface|Viewport|AddtoViewport _returnvalue 0))

(fn Movement
  (params (A :type Float%20%28double-precision%29) (ScaleValue :type Float%20%28single-precision%29))
  (Pawn|Input|AddMovementInput "0.800000,0.000000,0.000000" ScaleValue false)
  (Pawn|SetControlRotation (Pawn|GetController) (select (> A 0.0) (Math|Rotator|MakeRotator 0.0 0.0 0.0) (Math|Rotator|MakeRotator 0.0 0.0 1.8e+02))))

(fn Damage
  (params (B :type Float%20%28double-precision%29) (self2 :type Paper%20Flipbook%20Component%20Object%20Reference))
  (Variables|Default|SetHealth (- (Variables|Default|GetHealth) B))
  (if (<= (Variables|Default|GetHealth) 0.0)
    (Sprite|SetFlipbook (Variables|Default|GetSprite) "/Game/Blueprints/Player/Bosses/Royal_Executioner/Pixel/Sprites/Death/Death1.Death1")
    (Components|Timeline|SetLooping (Variables|Default|GetSprite) false)
    (Variables|Default|SetIsDead true)
    (else
      (Sprite|SetFlipbook (Variables|Default|GetSprite) "/Game/Blueprints/Player/Bosses/Royal_Executioner/Pixel/Sprites/Hurt/Hurt1.Hurt1")
      (Components|Timeline|SetLooping self2 false))))

(fn VoidTP
  (if (Variables|Default|GetHasVoidTelport)
    (Transformation|Teleport "21860.000000,0.000000,-3570.000000" "0, 0, 0")))

(fn SpawnArrow
  (bind _returnvalue (Transformation|GetActorLocation))
  (bind _returnvalue_2 (Actor|GetActorOfClass "/Game/Blueprints/Player/Attack/Arrow.Arrow_C"))
  (if (Variables|Default|GetIs%20Double%20Jumping)
    (if (Variables|Default|GetPlacePLatform)
      (if (> (Variables|Default|GetSpawnablePLatforms) 0)
        (Transformation|SetActorLocation _returnvalue_2 (Math|Vector|MakeVector (.x _returnvalue) (.y _returnvalue) (- (.z _returnvalue) 5e+01)) false true)))))

(fn CheckforOut)